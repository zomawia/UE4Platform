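; CowardEnemy_bp is an enemy driven by a string STATE, starting idle and switching to attack when PawnSensing sees FFPlayer_bp.
; Tick branches on state: attack plays a looping animation and spawns Bullets behind a Delay.
; Stunned and lifted enable physics and query-only capsule collision, with stunned also changing animation; neither state is set here.
; Viewport-top bouncing and start-position logic are disconnected.
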(event OnSeePawn(PawnSensing)
  (params (Pawn :type Pawn%20Object%20Reference))
  ;[1 1 1] go to attack if pawn is seent
  (Utilities|Casting|CastToFFPlayer_bp Pawn)
  (if (Utilities|Enum|Equal(Enum) (Variables|Default|GetSTATE) (Utilities|String|MakeLiteralString "IDLE"))
    (Variables|Default|SetSTATE "ATTACK")))

(event EventBeginPlay
  ;[1 1 1] store window size
  (Variables|Default|SetSTATE "IDLE")
  (bind _output_get (Variables|Default|Setviewport (Viewport|GetViewportSize)))
  (Development|PrintString (Utilities|String|ToString(Vector2d) _output_get)))

(event Collision|EventActorBeginOverlap
  (params (OtherActor :type Actor%20Object%20Reference)))

(event EventTick
  (params (DeltaSeconds :type Float%20%28single-precision%29))
  (bind _capsule (Variables|Default|GetCapsule))
  (switch string (Variables|Default|GetSTATE)
    (:ATTACK
      (Utilities|FlowControl|Delay 2.0)
      ;[1 1 1] spawn bullets
      (Class|SkinnedMeshComponent|SetSkeletalMesh (Variables|Default|GetSkeletalMesh) 0 true)
      (Components|Animation|PlayAnimation (Variables|Default|GetSkeletalMesh) 0 true)
      (if (Utilities|Enum|Equal(Enum) (Variables|Default|GetSTATE) (Utilities|String|MakeLiteralString "ATTACK"))
        (Game|SpawnActorfromClass "/Game/FF/Blueprints/Bullet.Bullet_C" (Transformation|GetActorTransform) "Undefined" 0 0)))
    (:STUNNED
      (Physics|SetSimulatePhysics _capsule true)
      (Components|Animation|PlayAnimation (Variables|Default|GetSkeletalMesh) "/Game/FF/Animations/BALLS.BALLS" true)
      (Collision|SetCollisionEnabled (Variables|Default|GetCapsule) "QueryOnly" :!label _label))
    (:LIFTED
      (Physics|SetSimulatePhysics _capsule true)
      (goto _label))))

(fn ConstructionScript)