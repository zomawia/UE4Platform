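; Basic enemy driven by a STATE string evaluated every Tick: idle, attack, stunned or lifted.
; Pawn sensing switches it from idle to attack on seeing the player, then a Tick-driven Delay spaces out bullet spawns.
; Stunned and lifted enable mesh physics; stunned also flips vertical velocity at the top screen edge, throttled by a resetting DoOnce.
; Nothing here sets the stunned or lifted states.
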(event OnSeePawn(PawnSensing)
  (params (Pawn :type Pawn%20Object%20Reference))
  ;[1 1 1] go to attack if pawn is seent
  (Utilities|Casting|CastToFFPlayer_bp Pawn)
  (if (Utilities|Enum|Equal(Enum) (Variables|Default|GetSTATE) (Utilities|String|MakeLiteralString "IDLE"))
    (Variables|Default|SetSTATE "ATTACK")))

(event EventBeginPlay
  ;[1 1 1] store window size
  (Variables|Default|SetSTATE "IDLE")
  (bind _output_get (Variables|Default|Setviewport (Viewport|GetViewportSize)))
  (Development|PrintString (Utilities|String|ToString(Vector2d) _output_get)))

(event Collision|EventActorBeginOverlap
  (params (OtherActor :type Actor%20Object%20Reference)))

(event EventTick
  (params (DeltaSeconds :type Float%20%28single-precision%29))
  (bind _skeletalmesh (Variables|Default|GetSkeletalMesh))
  (switch string (Variables|Default|GetSTATE)
    (:IDLE
      (Components|Animation|PlayAnimation (Variables|Default|GetSkeletalMesh) "/Game/FF/Animations/BALLS.BALLS" false))
    (:ATTACK
      ;[1 1 1] spawn bullets
      (Utilities|FlowControl|Delay 2.0)
      (if (Utilities|Enum|Equal(Enum) (Variables|Default|GetSTATE) (Utilities|String|MakeLiteralString "ATTACK"))
        (Game|SpawnActorfromClass "/Game/FF/Blueprints/Bullet.Bullet_C" (Transformation|GetActorTransform) "Undefined" 0 0)))
    (:STUNNED
      (Physics|SetSimulatePhysics _skeletalmesh true)
      (Components|Animation|PlayAnimation _skeletalmesh "/Game/FF/Animations/BALLS.BALLS" true)
      ;[1 1 1] reflect off camera dimensions
      (bind _output_get (Variables|Default|SetscreenPos (.ScreenPosition (Class|GameplayStatics|ProjectWorldtoScreen (Game|GetPlayerController 0) (Transformation|GetActorLocation) true))))
      (if (and (Physics|IsSimulatingPhysics (Variables|Default|GetSkeletalMesh) "None") (< (.Y (Math|Vector2D|BreakVector2D _output_get)) 2.0))
        (Utilities|FlowControl|DoOnce false :!label _label
          (:Completed
            (Physics|SetPhysicsLinearVelocity (Variables|Default|GetSkeletalMesh) (* (Transformation|GetVelocity) (Math|Vector|MakeVector 1.0 1.0 -1.0)) false "None")
            (Utilities|FlowControl|Delay 2.0)
            (goto _label Reset)))))
    (:LIFTED
      (Physics|SetSimulatePhysics _skeletalmesh true))))

(fn ConstructionScript)